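; Base actor for a grid tile in a TileMap, with overridable hooks for player entry and next-tile lookup.
; FindNeighbours links the tile to adjacent tiles in four directions.
; ChangeTileType swaps it for a spawned tile of another class, relinking neighbours, updating the map and refreshing DirectionTile directions, then destroys itself.
; ChangePlayer cycles possession through PlayerParty actors using the map's shared index.
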(event Custom|OnEnter
  (params (PlayerPawn :type Player%20Party%20Object%20Reference) (FromTile :type Tile%20Object%20Reference)))

(fn ConstructionScript)

(fn SetNeighbour
  (params (Direction :type Direction%20Object%20Reference) (NewNeighbour :type Tile%20Object%20Reference))
  (Utilities|Map|Add (Variables|Default|GetNeighbours) Direction NewNeighbour))

(fn FindNeighbours
  (bind _coord (Variables|Default|GetCoord))
  (for _array_element (Utilities|Array|MakeArray "/Game/Blueprints/Up.Up" "/Game/Blueprints/Down.Down" "/Game/Blueprints/Left.Left" "/Game/Blueprints/Right.Right")
    (if (Default|IsCoordinRange (Variables|Default|GetTileMap) (Utilities|Struct|MakeCoord (+ (.x _coord) (.x (Variables|/Game/Blueprints/Direction.Direction_C|GetDelta _array_element))) (+ (.y _coord) (.y (Variables|/Game/Blueprints/Direction.Direction_C|GetDelta _array_element)))))
      (Utilities|IsValid (Default|GetTileatCoord (Variables|Default|GetTileMap) (Utilities|Struct|MakeCoord (+ (.x _coord) (.x (Variables|/Game/Blueprints/Direction.Direction_C|GetDelta _array_element))) (+ (.y _coord) (.y (Variables|/Game/Blueprints/Direction.Direction_C|GetDelta _array_element)))))
        (:Is%20Valid
          (Utilities|Map|Add (Variables|Default|GetNeighbours) _array_element (Default|GetTileatCoord (Variables|Default|GetTileMap) (Utilities|Struct|MakeCoord (+ (.x _coord) (.x (Variables|/Game/Blueprints/Direction.Direction_C|GetDelta _array_element))) (+ (.y _coord) (.y (Variables|/Game/Blueprints/Direction.Direction_C|GetDelta _array_element)))))))))))

(fn ChangeTileType
  (if (and (Utilities|IsValidClass (Variables|Default|GetNewTileType)) (!= (Variables|Default|GetNewTileType) (Utilities|GetClass self)))
    (bind _returnvalue (Game|SpawnActorfromClass (Variables|Default|GetNewTileType) (Transformation|GetActorTransform) "AlwaysSpawn" 0 (Variables|Default|GetCoord) (Variables|Default|GetNeighbours) (Variables|Default|GetTileMap) (Variables|Default|GetNewTileType) 0))
    (LocalVariables|SetSpawnedTile _returnvalue)
    (bind _keys (Utilities|Map|Keys (Variables|Default|GetNeighbours)))
    (for _array_element _keys
      (Utilities|IsValid (.Value (Utilities|Map|Find (Variables|Default|GetNeighbours) _array_element))
        (:Is%20Valid
          (CallFunction|SetNeighbour (.Value (Utilities|Map|Find (Variables|Default|GetNeighbours) _array_element)) (Variables|/Game/Blueprints/Direction.Direction_C|GetOppositeDirection _array_element) (LocalVariables|GetSpawnedTile))
          (Transformation|AttachActorToActor (LocalVariables|GetSpawnedTile) (Variables|Default|GetTileMap) "None" "KeepWorld" "KeepWorld" "KeepWorld" true)
          (Default|ReplaceTile (Variables|Default|GetTileMap) (LocalVariables|GetSpawnedTile)))))
    (if (== (Utilities|GetClass (LocalVariables|GetSpawnedTile)) "/Game/Blueprints/Tiles/DirectionTile.DirectionTile_C")
      (bind _asdirection_tile (Utilities|Casting|CastToDirectionTile (LocalVariables|GetSpawnedTile)))
      (Default|SetDirections _asdirection_tile))
    (Actor|DestroyActor)))

(fn CanPlayerEnter
  (params (PlayerPawn :type Player%20Party%20Object%20Reference) (TileFrom :type Tile%20Object%20Reference))
  (return false))

(fn GetNextTile
  (params (PlayerPawn :type Player%20Party%20Object%20Reference) (FromTile :type Tile%20Object%20Reference))
  (return 0))

(fn ChangePlayer
  (Math|Integer|IncrementInt (Variables|/Game/Blueprints/TileMap.TileMap_C|GetCurrent%20Index (Variables|Default|GetTileMap))
    (:%20%20
      (bind _outactors (Actor|GetAllActorsOfClass "/Game/Blueprints/PlayerParty.PlayerParty_C"))
      (bind _output_get (LocalVariables|SetPlayerPartyActors _outactors))
      (if (== (Variables|/Game/Blueprints/TileMap.TileMap_C|GetCurrent%20Index (Variables|Default|GetTileMap)) (Utilities|Array|Length _outactors))
        (Variables|/Game/Blueprints/TileMap.TileMap_C|SetCurrent%20Index (Variables|Default|GetTileMap) 0))
      (Pawn|Possess (Game|GetPlayerController 0) (Utilities|Array|Get(acopy) _output_get (Variables|/Game/Blueprints/TileMap.TileMap_C|GetCurrent%20Index (Variables|Default|GetTileMap)))))))