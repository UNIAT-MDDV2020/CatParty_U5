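; Game Instance for a Mario Party-style game that holds per-player board state and the current level map.
; Parallel arrays indexed by player store tile location, coins, stars, direction and tile coordinate.
; Get and set functions read or overwrite a player's full record, saving the tile actor's world location rather than the actor itself.
; A separate update function adds coin and star deltas to the stored totals.
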(fn GetPlayerData
  (params (Player :type Integer))
  (return (Utilities|Array|Get(acopy) (Variables|Default|GetPlayerTileLocation) Player) (Utilities|Array|Get(acopy) (Variables|Default|GetPlayerCoins) Player) (Utilities|Array|Get(acopy) (Variables|Default|GetPlayerStars) Player) (Utilities|Array|Get(acopy) (Variables|Default|GetPlayerDirection) Player) (Utilities|Array|Get(acopy) (Variables|Default|GetPlayerTileCoord) Player)))

(fn SetPlayerData
  (params (Player :type Integer) (Tile :type Tile%20Object%20Reference) (Coins :type Integer) (Stars :type Integer) (Direction :type Direction%20Object%20Reference) (TileCoord :type Coord%20Structure))
  (Utilities|Array|SetArrayElem (Variables|Default|GetPlayerTileLocation) Player (Transformation|GetActorLocation Tile) true)
  (Utilities|Array|SetArrayElem (Variables|Default|GetPlayerCoins) Player Coins true)
  (Utilities|Array|SetArrayElem (Variables|Default|GetPlayerStars) Player Stars true)
  (Utilities|Array|SetArrayElem (Variables|Default|GetPlayerDirection) Player Direction true)
  (Utilities|Array|SetArrayElem (Variables|Default|GetPlayerTileCoord) Player TileCoord true)
  (Development|PrintString "Player Data Saved"))

(fn UpdatePlayerData
  (params (Player :type Integer) (CoinsToAdd :type Integer) (StarsToAdd :type Integer))
  (bind _playercoins (Variables|Default|GetPlayerCoins))
  (bind _playerstars (Variables|Default|GetPlayerStars))
  (Utilities|Array|SetArrayElem _playercoins Player (+ (Utilities|Array|Get(acopy) _playercoins Player) CoinsToAdd))
  (Utilities|Array|SetArrayElem _playerstars Player (+ (Utilities|Array|Get(acopy) _playerstars Player) StarsToAdd)))

(fn SetLevelData
  (params (CurrentLevel :type Name))
  (Variables|Default|SetLevelMap CurrentLevel))

(fn GetLevelData
  (return (Variables|Default|GetLevelMap)))