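; Ice tile Blueprint that makes a player pawn keep sliding in a straight line across it.
; GetNextTile finds the direction of the tile the pawn came from in the Neighbours map and returns the neighbour in the opposite direction, or nothing if no match is found.
; CanPlayerEnter always allows entry, and the event graph holds only disabled default events.
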(event EventBeginPlay)

(event Collision|EventActorBeginOverlap
  (params (OtherActor :type Actor%20Object%20Reference)))

(event EventTick
  (params (DeltaSeconds :type Float%20%28single-precision%29)))

(fn ConstructionScript
  (|CallParentFunction))

(fn GetNextTile
  (params (PlayerPawn :type Player%20Party%20Object%20Reference) (FromTile :type Tile%20Object%20Reference))
  (bind _neighbours (Variables|Default|GetNeighbours))
  (bind _keys (Utilities|Map|Keys (Variables|Default|GetNeighbours)))
  (for _array_element _keys
    (if (== (.Value (Utilities|Map|Find _neighbours _array_element)) FromTile)
      (return (.Value (Utilities|Map|Find _neighbours (Variables|/Game/Blueprints/Direction.Direction_C|GetOppositeDirection _array_element))))))
  (return 0))

(fn CanPlayerEnter
  (params (PlayerPawn :type Player%20Party%20Object%20Reference) (TileFrom :type Tile%20Object%20Reference))
  (return true))