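; Direction tile that halts a player pawn on entry and works out which directions lead onward.
; SetDirections builds its move map from a forced direction if one is valid, otherwise from every neighbour the player can enter.
; On entry it disables pawn movement, copies that map and removes the direction opposite the pawn's current one, ruling out backtracking.
; The tile itself always allows entry.
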(event EventOnEnter
  (params (PlayerPawn :type Player%20Party%20Object%20Reference) (FromTile :type Tile%20Object%20Reference))
  ;[1 0.2109 0] Remove Opposite Tile
  (Variables|/Game/Blueprints/PlayerParty.PlayerParty_C|SetCanMove PlayerPawn false)
  (Variables|Default|SetPossibleMovieDirections (Variables|Default|GetMoveDirections))
  (bind _keys (Utilities|Map|Keys (Variables|Default|GetPossibleMovieDirections)))
  (for _array_element _keys
    (if (== _array_element (Variables|/Game/Blueprints/Direction.Direction_C|GetOppositeDirection (Variables|/Game/Blueprints/PlayerParty.PlayerParty_C|GetCurrentDirection PlayerPawn)))
      (Utilities|Map|Remove (Variables|Default|GetPossibleMovieDirections) _array_element))))

(fn ConstructionScript
  (|CallParentFunction))

(fn CanPlayerEnter
  (params (PlayerPawn :type Player%20Party%20Object%20Reference) (TileFrom :type Tile%20Object%20Reference))
  (return true))

(fn SetDirections
  (bind _forcedirection (Variables|Default|GetForceDirection))
  (Variables|Default|SetMoveDirections (LocalVariables|GetEmptyMap))
  (Utilities|IsValid (Variables|Default|GetForceDirection)
    (:Is%20Valid
      (Utilities|Map|Add (Variables|Default|GetMoveDirections) _forcedirection (.Value (Utilities|Map|Find (Variables|Default|GetNeighbours) _forcedirection))))
    (:Is%20Not%20Valid
      (bind _values (Utilities|Map|Values (Variables|Default|GetNeighbours)))
      (for (_array_element _array_index) _values
        (if (CallFunction|CanPlayerEnter _array_element)
          (bind _keys (Utilities|Map|Keys (Variables|Default|GetNeighbours)))
          (Utilities|Map|Add (Variables|Default|GetMoveDirections) (Utilities|Array|Get(acopy) _keys _array_index) _array_element))))))