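; Character display actor for a selection scene, previewing cat skins on a skeletal mesh alongside a slowly spinning cube.
; BeginPlay adds the Character_selecionScene widget, shows the mouse cursor and caches the CatAnim instance.
; SetCharacter swaps the mesh from CatsSkinMesh by index, unhides it and flags IsSelected on its anim instance.
; Show and hide events toggle the Abyss cat and cube; the other spawn events are empty.
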(event Custom|CubeSpawn)

(event Custom|BobtailSpawn)

(event Custom|BlueSpawn)

(event Custom|BlackWhiteSpawn)

(event Custom|CubeShow
  (Development|SetHiddeninGame (Variables|Default|GetCube) false false))

(event Custom|CubeHide
  (Development|SetHiddeninGame (Variables|Default|GetCube) true false))

(event Custom|CAbysShow
  (CallFunction|SetCharacter))

(event Custom|CAbysHide
  (Development|SetHiddeninGame (Variables|Default|GetSkeletal_CAbyss) true false))

(event EventBeginPlay
  (bind _returnvalue (UserInterface|CreateWidget "/Game/HUD/Character_selecionScene.Character_selecionScene_C"))
  (bind _output_get (Variables|Default|SetWidgetRef _returnvalue))
  (UserInterface|Viewport|AddtoViewport _output_get 0)
  ;[0.2409 0.04797 1] Mouse Selection
  (Variables|/Script/Engine.PlayerController|SetbShowMouseCursor (Game|GetPlayerController 0) true)
  (bind _ascat_anim (Utilities|Casting|CastToCatAnim (Components|SkeletalMesh|GetAnimInstance (Variables|Default|GetSkeletal_CAbyss))))
  (Variables|Default|SetAs%20Cat%20Anim _ascat_anim))

(event Collision|EventActorBeginOverlap
  (params (OtherActor :type Actor%20Object%20Reference)))

(event EventTick
  (params (DeltaSeconds :type Float%20%28single-precision%29))
  (Transformation|AddLocalRotation (Variables|Default|GetCube) (Math|Rotator|MakeRotator 0.0 0.0 (+ DeltaSeconds 1.0)) false false))

(fn ConstructionScript)

(fn SetCharacter
  (params (Cat :type Integer))
  (bind _skeletal_cabyss (Variables|Default|GetSkeletal_CAbyss))
  (Class|SkinnedMeshComponent|SetSkeletalMesh _skeletal_cabyss (Utilities|Array|Get(acopy) (Variables|Default|GetcatsSkinMesh) Cat) true)
  (Development|SetHiddeninGame _skeletal_cabyss false false)
  (bind _ascat_anim (Utilities|Casting|CastToCatAnim (Components|SkeletalMesh|GetAnimInstance (Variables|Default|GetSkeletal_CAbyss))))
  (Variables|/Game/Blueprints/CatAnim.CatAnim_C|SetisSelected _ascat_anim true))