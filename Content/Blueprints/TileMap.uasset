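; Tile map actor for a board game with star, blue, red and direction tiles, which places player parties on a spawn tile at BeginPlay.
; ResetMap rebuilds a flat-indexed Width×Height grid of border and fill tiles, then links neighbours.
; AlignTiles recursively rotates tiles along the path from the spawn tile, branching at direction tiles.
; SpawnStar turns the current star tile blue or red and makes a random blue or red tile the star.
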(event EventBeginPlay
  (bind _returnvalue (Game|Player|GetPlayerPawn 3))
  (bind _returnvalue_2 (Game|Player|GetPlayerPawn 1))
  (bind _returnvalue_3 (Game|Player|GetPlayerPawn 2))
  (bind _returnvalue_4 (Game|Player|GetPlayerPawn 0))
  (CallFunction|SpawnPlayers)
  (Transformation|SetActorLocation _returnvalue_4 (Transformation|GetActorLocation (Variables|Default|GetPlayerSpawnTile)) false false)
  (Transformation|SetActorRotation _returnvalue_4 (Variables|/Game/Blueprints/Direction.Direction_C|GetRotation (Variables|Default|GetPlayerSpawnDirection)))
  (bind _asplayer_party (Utilities|Casting|CastToPlayerParty _returnvalue_4))
  (Variables|/Game/Blueprints/PlayerParty.PlayerParty_C|SetCurrentTile _asplayer_party (Variables|Default|GetPlayerSpawnTile))
  (Variables|/Game/Blueprints/PlayerParty.PlayerParty_C|SetCurrentDirection _asplayer_party (Variables|Default|GetPlayerSpawnDirection))
  (Transformation|SetActorLocation _returnvalue_2 (Transformation|GetActorLocation (Variables|Default|GetPlayerSpawnTile)) false false)
  (Transformation|SetActorRotation _returnvalue_2 (Variables|/Game/Blueprints/Direction.Direction_C|GetRotation (Variables|Default|GetPlayerSpawnDirection)))
  (bind _asplayer_party_2 (Utilities|Casting|CastToPlayerParty _returnvalue_2))
  (Variables|/Game/Blueprints/PlayerParty.PlayerParty_C|SetCurrentTile _asplayer_party_2 (Variables|Default|GetPlayerSpawnTile))
  (Variables|/Game/Blueprints/PlayerParty.PlayerParty_C|SetCurrentDirection _asplayer_party_2 (Variables|Default|GetPlayerSpawnDirection))
  (Transformation|SetActorLocation _returnvalue_3 (Transformation|GetActorLocation (Variables|Default|GetPlayerSpawnTile)) false false)
  (Transformation|SetActorRotation _returnvalue_3 (Variables|/Game/Blueprints/Direction.Direction_C|GetRotation (Variables|Default|GetPlayerSpawnDirection)))
  (bind _asplayer_party_3 (Utilities|Casting|CastToPlayerParty _returnvalue_3))
  (Variables|/Game/Blueprints/PlayerParty.PlayerParty_C|SetCurrentTile _asplayer_party_3 (Variables|Default|GetPlayerSpawnTile))
  (Variables|/Game/Blueprints/PlayerParty.PlayerParty_C|SetCurrentDirection _asplayer_party_3 (Variables|Default|GetPlayerSpawnDirection))
  (Transformation|SetActorLocation _returnvalue (Transformation|GetActorLocation (Variables|Default|GetPlayerSpawnTile)) false false)
  (Transformation|SetActorRotation _returnvalue (Variables|/Game/Blueprints/Direction.Direction_C|GetRotation (Variables|Default|GetPlayerSpawnDirection)))
  (bind _asplayer_party_4 (Utilities|Casting|CastToPlayerParty _returnvalue))
  (Variables|/Game/Blueprints/PlayerParty.PlayerParty_C|SetCurrentTile _asplayer_party_4 (Variables|Default|GetPlayerSpawnTile))
  (Variables|/Game/Blueprints/PlayerParty.PlayerParty_C|SetCurrentDirection _asplayer_party_4 (Variables|Default|GetPlayerSpawnDirection)))

(fn ConstructionScript)

(fn CoordtoIndex
  (params (Coord :type Coord%20Structure))
  (return (+ (.x Coord) (* (.y Coord) (Variables|Default|GetWidth)))))

(fn IndextoCoord
  (params (Index :type Integer))
  (bind _width (Variables|Default|GetWidth))
  (return (Utilities|Struct|MakeCoord (Math|Integer|%(Integer) Index _width) (/ Index _width))))

(fn IsCoordBorder
  (params (Coord :type Coord%20Structure))
  (return (Math|Boolean|ORBoolean (== (- (Variables|Default|GetWidth) 1) (.x Coord)) (== (.x Coord) 0) (== (.y Coord) 0) (== (- (Variables|Default|GetHeight) 1) (.y Coord)))))

(fn IsCoordinRange
  (params (Coord :type Coord%20Structure))
  (return (not (Math|Boolean|ORBoolean (>= (.x Coord) (Variables|Default|GetWidth)) (< (.x Coord) 0) (< (.y Coord) 0) (>= (.y Coord) (Variables|Default|GetHeight))))))

(fn GetTileatCoord
  (params (Coord :type Coord%20Structure))
  (return (Utilities|Array|Get(acopy) (Variables|Default|GetTiles) (CallFunction|CoordtoIndex Coord))))

(fn ResetMap
  (bind _tiles (Variables|Default|GetTiles))
  (for _array_element _tiles
    (Utilities|IsValid _array_element
      (:Is%20Valid
        (Actor|DestroyActor _array_element))))
  (Utilities|Array|Clear _tiles)
  (for _index (range 0 (- (Variables|Default|GetHeight) 1)) ; Y
    (for _index_2 (range 0 (- (Variables|Default|GetWidth) 1)) ; X
      (bind _returnvalue (Game|SpawnActorfromClass (select (CallFunction|IsCoordBorder (Utilities|Struct|MakeCoord _index_2 _index)) (Variables|Default|GetBorderTileType) (Variables|Default|GetFillTileType)) (Math|Transform|MakeTransform (Math|Vector|MakeVector (* _index 1e+02) (* _index_2 1e+02) 0.0) "0, 0, 0" "1,1,1") "Undefined" 0 (Utilities|Struct|MakeCoord _index_2 _index) 0 self (select (CallFunction|IsCoordBorder (Utilities|Struct|MakeCoord _index_2 _index)) (Variables|Default|GetBorderTileType) (Variables|Default|GetFillTileType)) 0))
      (Utilities|Array|Add (Variables|Default|GetTiles) _returnvalue)
      (Transformation|AttachActorToActor _returnvalue self "None" "KeepWorld" "KeepWorld" "KeepWorld" true)))
  (for _array_element_2 (Variables|Default|GetTiles)
    (Default|FindNeighbours _array_element_2)))

(fn ReplaceTile
  (params (NewTile :type Tile%20Object%20Reference))
  (Utilities|Array|SetArrayElem (Variables|Default|GetTiles) (CallFunction|CoordtoIndex (Variables|/Game/Blueprints/Tile.Tile_C|GetCoord NewTile)) NewTile))

(fn AlignTiles
  (Utilities|IsValid (Variables|Default|GetTileToRotate)
    (:Is%20Valid
      (if (not (Variables|/Game/Blueprints/Tile.Tile_C|GetIsAligned (Variables|Default|GetTileToRotate)))
        (bind _returnvalue (Transformation|SetActorRotation (Variables|Default|GetTileToRotate) (CallFunction|DirectiontoAlignRotation (Variables|Default|GetDirectionToRotate)) :!label _label))
        (if _returnvalue
          (LocalVariables|SetNextTile (.Value (Utilities|Map|Find (Variables|/Game/Blueprints/Tile.Tile_C|GetNeighbours (Variables|Default|GetTileToRotate)) (Variables|Default|GetDirectionToRotate))))
          (Variables|/Game/Blueprints/Tile.Tile_C|SetIsAligned (Variables|Default|GetTileToRotate) true)
          (if (Math|Boolean|ORBoolean (== (Utilities|GetClass (LocalVariables|GetNextTile)) "/Game/Blueprints/Tiles/BlueTile.BlueTile_C") (== (Utilities|GetClass (LocalVariables|GetNextTile)) "/Game/Blueprints/Tiles/RedTile.RedTile_C") (== (Utilities|GetClass (LocalVariables|GetNextTile)) "/Game/Blueprints/Tiles/StarTile.StarTile_C"))
            (Variables|Default|SetTileToRotate (LocalVariables|GetNextTile))
            (CallFunction|AlignTiles)
            (elif (== (Utilities|GetClass (LocalVariables|GetNextTile)) "/Game/Blueprints/Tiles/DirectionTile.DirectionTile_C")
              (bind _keys (Utilities|Map|Keys (Variables|/Game/Blueprints/Tile.Tile_C|GetMoveDirections (LocalVariables|GetNextTile))))
              (for _array_element _keys
                (Variables|Default|SetDirectionToRotate _array_element)
                (Variables|Default|SetTileToRotate (.Value (Utilities|Map|Find (Variables|/Game/Blueprints/Tile.Tile_C|GetNeighbours (LocalVariables|GetNextTile)) (Variables|Default|GetDirectionToRotate))))
                (CallFunction|AlignTiles)))))))
    (:Is%20Not%20Valid
      ;[0.5 1 0] Only works in 1st call
      (Variables|Default|SetTileToRotate (Variables|Default|GetPlayerSpawnTile))
      (Variables|Default|SetDirectionToRotate (Variables|Default|GetPlayerSpawnDirection))
      (goto _label))))

(fn DirectiontoAlignRotation
  (params (Direction :type Direction%20Object%20Reference))
  (if (== Direction "/Game/Blueprints/Up.Up")
    (Variables|Default|SetRotator "0,90.000000, 0")
    (return (Variables|Default|GetRotator))
    (elif (== Direction "/Game/Blueprints/Down.Down")
      (Variables|Default|SetRotator "0,270.000000, 0")
      (return (Variables|Default|GetRotator))
      (elif (== Direction "/Game/Blueprints/Right.Right")
        (Variables|Default|SetRotator "0,180.000000, 0")
        (return (Variables|Default|GetRotator))
        (elif (== Direction "/Game/Blueprints/Left.Left")
          (Variables|Default|SetRotator "0, 0, 0")
          (return (Variables|Default|GetRotator)))))))

(fn ResetTileRotation
  (for _array_element (Variables|Default|GetTiles)
    (Variables|/Game/Blueprints/Tile.Tile_C|SetIsAligned _array_element false)
    (Transformation|SetActorRotation _array_element)
    (Variables|Default|SetTileToRotate (Variables|Default|GetPlayerSpawnTile))
    (Variables|Default|SetDirectionToRotate (Variables|Default|GetPlayerSpawnDirection))
    (Development|PrintString (Utilities|GetDisplayName _array_element))))

(fn SpawnStar
  (bind _array_element (Utilities|Array|ForEachLoopwithBreak (Variables|Default|GetTiles) :!label _label)
    (:LoopBody
      (if (== (Utilities|GetClass _array_element) "/Game/Blueprints/Tiles/StarTile.StarTile_C")
        (if (> (Math|Random|RandomFloat) 0.8)
          ;[1 0 0.7734] Possible tiles to overwrite
          (Variables|/Game/Blueprints/Tile.Tile_C|SetNewTileType _array_element "/Game/Blueprints/Tiles/RedTile.RedTile_C")
          (else
            (Variables|/Game/Blueprints/Tile.Tile_C|SetNewTileType _array_element "/Game/Blueprints/Tiles/BlueTile.BlueTile_C")))
        (Default|ChangeTileType _array_element)
        (LocalVariables|SetStarIsSet true)
        (bind _filteredarray (Utilities|Array|FilterArray (Variables|Default|GetTiles) "/Game/Blueprints/Tiles/BlueTile.BlueTile_C" :!label _label_2))
        (bind _filteredarray_2 (Utilities|Array|FilterArray (Variables|Default|GetTiles) "/Game/Blueprints/Tiles/RedTile.RedTile_C"))
        (Utilities|Array|AppendArray _filteredarray _filteredarray_2)
        (bind _astile (Utilities|Casting|CastToTile (Utilities|Array|Get(acopy) _filteredarray (Math|Random|RandomInteger (Utilities|Array|Length _filteredarray)))))
        (Variables|/Game/Blueprints/Tile.Tile_C|SetNewTileType _astile "/Game/Blueprints/Tiles/StarTile.StarTile_C")
        (Default|ChangeTileType _astile)
        (goto _label Break)))
    (:Completed
      (if (not (LocalVariables|GetStarIsSet))
        (goto _label_2)))))

(fn SpawnPlayers
  (bind _outactors (Actor|GetAllActorsOfClass "/Script/Engine.PlayerStart"))
  (Variables|Default|SetPlayersStartArray _outactors)
  (for _index (range 0 (- (LocalVariables|GetMaxPlayerCount) 1))
    (LocalVariables|SetIndex _index)
    (for _array_element (Variables|Default|GetPlayersStartArray)
      (if (Utilities|Name|Equal(Name) (Variables|/Script/Engine.PlayerStart|GetPlayerStartTag _array_element) (Utilities|String|StringToName (Utilities|String|ToString(Integer) (LocalVariables|GetIndex))))
        (Class|GameplayStatics|CreatePlayer (LocalVariables|GetIndex))
        (Pawn|Possess (Game|GetPlayerController (LocalVariables|GetIndex)))
        (Utilities|Array|AddUnique (Variables|Default|GetPlayers) 0)))))