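; Player pawn for a Mario Party-style board game, handling dice rolls, tile movement and end-of-turn effects.
; A roll counts down as timelines move and rotate the pawn along tile neighbours, with a delayed polling loop awaiting directional input at junctions.
; The landing tile adjusts coins or opens the star shop.
; Coin tiles also save player data to the game instance, pass the turn and load the minigame when the index wraps.
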(event Custom|MoveTo
  (params (TileToMove :type Tile%20Object%20Reference))
  ;[0.7812 0 1] Player movement
  (Utilities|IsValid TileToMove
    (:Is%20Valid
      (if (Default|CanPlayerEnter TileToMove self (Variables|Default|GetCurrentTile))
        (Variables|Default|SetTargetTile (Variables|Default|GetCurrentTile))
        (bind _moveto (Timeline|Timeline_1 PlayFromStart)
          (:Update
            (Variables|Default|SetIsWalking true)
            (Transformation|SetActorLocation (Math|Vector|Lerp(Vector) (Transformation|GetActorLocation (Variables|Default|GetCurrentTile)) (Transformation|GetActorLocation TileToMove) _moveto) false false))
          (:Finished
            (Variables|Default|SetIsWalking false)
            (Variables|Default|SetTemp (Variables|Default|GetCurrentTile))
            (Variables|Default|SetCurrentTile TileToMove)
            (bind _output_get (Variables|Default|SetTargetTile (Default|GetNextTile (Variables|Default|GetCurrentTile) self (Variables|Default|GetTemp))))
            (Utilities|IsValid _output_get
              (:Is%20Valid
                (if (Default|CanPlayerEnter _output_get self (Variables|Default|GetCurrentTile))
                  (CallFunction|Moveto (Variables|Default|GetTargetTile))))
              (:Is%20Not%20Valid
                (Variables|Default|SetTargetTile 0)))
            (Default|OnEnter (Variables|Default|GetCurrentTile) self (Variables|Default|GetTemp))))))))

(event Custom|RotateToDirection
  (params (Direction :type Direction%20Object%20Reference))
  ;[0 1 0.8125] Player Rotation
  (Utilities|IsValid Direction
    (:Is%20Valid
      (Variables|Default|SetTargetDirection Direction)
      (bind _newtrack_0 (Timeline|Timeline_0 PlayFromStart)
        (:Update
          (Transformation|SetActorRotation (Math|Rotator|Lerp(Rotator) (Variables|/Game/Blueprints/Direction.Direction_C|GetRotation (Variables|Default|GetCurrentDirection)) (Variables|/Game/Blueprints/Direction.Direction_C|GetRotation (Variables|Default|GetTargetDirection)) _newtrack_0)))
        (:Finished
          (bind _output_get (Variables|Default|SetCurrentDirection (Variables|Default|GetTargetDirection)))
          (Variables|Default|SetTargetDirection _output_get))))))

(event EventBeginPlay
  (Rendering|SetVisibility (Variables|Default|GetdiceNumber) false false)
  (bind _outactors (Actor|GetAllActorsOfClass "PlayerParty_C"))
  (Variables|PlayerParty_C|SetActual%20Player (Utilities|Array|Get(acopy) _outactors) true))

(event Input|ActionEvents|InputActionDice
  (params (Key :type Key%20Structure))
  ;[1 0.9844 0] Dice Movement
  (:Pressed
    (if (not (Variables|Default|GetIsMoving))
      (Rendering|SetVisibility (Variables|Default|GetdiceNumber) true false)
      (Variables|Default|SetIsMoving true)
      (Variables|Default|SetActual%20Player true)
      (Variables|Default|SetMoveIndex (Math|Random|RandomIntegerinRange 1 10))
      (if (== (Variables|Default|GetMoveIndex) 0) :!label _label
        (Variables|Default|SetTargetDirection (Variables|Default|GetEmptyDirection) :!label _label_2)
        (if (== (Utilities|GetClass (Variables|Default|GetCurrentTile)) "/Game/Blueprints/Tiles/DirectionTile.DirectionTile_C")
          (bind _asdirection_tile (Utilities|Casting|CastToDirectionTile (Variables|Default|GetCurrentTile)))
          (bind _keys (Utilities|Map|Keys (Variables|/Game/Blueprints/Tiles/DirectionTile.DirectionTile_C|GetPossibleMovieDirections _asdirection_tile)))
          (if (== (Utilities|Array|Length _keys) 1) :!label _label_3
            (Variables|Default|SetTargetDirection (Utilities|Array|Get(acopy) _keys))
            (Variables|Default|SetCanMove true :!label _label_4)
            (Variables|Default|SetCurrentDirection (Variables|Default|GetTargetDirection))
            (CallFunction|Moveto (.Value (Utilities|Map|Find (Variables|/Game/Blueprints/Tile.Tile_C|GetNeighbours (Variables|Default|GetCurrentTile)) (Variables|Default|GetCurrentDirection))) :!label _label_5)
            (CallFunction|RotatetoDirection (Variables|Default|GetCurrentDirection))
            (Utilities|FlowControl|Delay 0.2)
            (goto _label)
            (else
              (Variables|Default|SetDirectionSelected false)
              (for _array_element _keys
                (if (== (Variables|Default|GetTargetDirection) _array_element)
                  (if (not (Variables|Default|GetDirectionSelected))
                    (Variables|Default|SetDirectionSelected true)
                    (goto _label_4))))
              (Utilities|FlowControl|Delay 0.1)
              (if (not (Variables|Default|GetDirectionSelected))
                (goto _label_3))))
          (else
            (Variables|Default|SetIsMoving false)
            (CallFunction|CheckTile)
            (Rendering|SetVisibility (Variables|Default|GetdiceNumber) false false)))
        (elif (Variables|Default|GetCanMove)
          (Rendering|Components|TextRender|SetText (Variables|Default|GetdiceNumber) (Utilities|Text|ToText(Integer) (Variables|Default|GetMoveIndex)))
          (Math|Integer|DecrementInt (Variables|Default|GetMoveIndex)
            (:%20%20
              (Utilities|IsValid (Variables|Default|GetTargetTile)
                (:Is%20Not%20Valid
                  (Utilities|IsValid (.Value (Utilities|Map|Find (Variables|/Game/Blueprints/Tile.Tile_C|GetNeighbours (Variables|Default|GetCurrentTile)) (Variables|Default|GetCurrentDirection)))
                    (:Is%20Valid
                      (goto _label_5)))))))
          (else
            (goto _label_2)))))))

(event Input|ActionEvents|InputActionMoveLeft
  (params (Key :type Key%20Structure))
  ;[0.1953 1 0] Player Map Input
  (:Pressed
    (if (== (Utilities|GetClass (Variables|Default|GetCurrentTile)) "/Game/Blueprints/Tiles/DirectionTile.DirectionTile_C")
      (Variables|Default|SetTargetDirection "/Game/Blueprints/Left.Left"))))

(event Input|ActionEvents|InputActionMoveRight
  (params (Key :type Key%20Structure))
  ;[0.1953 1 0] Player Map Input
  (:Pressed
    (if (== (Utilities|GetClass (Variables|Default|GetCurrentTile)) "/Game/Blueprints/Tiles/DirectionTile.DirectionTile_C")
      (Variables|Default|SetTargetDirection "/Game/Blueprints/Right.Right"))))

(event Input|ActionEvents|InputActionMoveUp
  (params (Key :type Key%20Structure))
  ;[0.1953 1 0] Player Map Input
  (:Pressed
    (if (== (Utilities|GetClass (Variables|Default|GetCurrentTile)) "/Game/Blueprints/Tiles/DirectionTile.DirectionTile_C")
      (Variables|Default|SetTargetDirection "/Game/Blueprints/Up.Up"))))

(event Input|ActionEvents|InputActionMoveDown
  (params (Key :type Key%20Structure))
  ;[0.1953 1 0] Player Map Input
  (:Pressed
    (if (== (Utilities|GetClass (Variables|Default|GetCurrentTile)) "/Game/Blueprints/Tiles/DirectionTile.DirectionTile_C")
      (Variables|Default|SetTargetDirection "/Game/Blueprints/Down.Down"))))

(fn ConstructionScript)

(fn CheckTile
  (bind _currenttile (Variables|Default|GetCurrentTile))
  (if (== (Utilities|GetClass (Variables|Default|GetCurrentTile)) "/Game/Blueprints/Tiles/BlueTile.BlueTile_C")
    (bind _output_get (Variables|Default|SetCoins (+ (Variables|Default|GetCoins) 3)))
    (Development|PrintString (Utilities|String|Append "Ganaste 3 Monedas tienes" (Utilities|String|ToString(Integer) _output_get)))
    ;[0.3008 0.2867 1] Change Player
    (bind _outactors (Actor|GetAllActorsOfClass "/Game/Blueprints/TileMap.TileMap_C" :!label _label))
    (Variables|Default|SetTileMap (Utilities|Array|Get(acopy) _outactors))
    ;[0.952 0.1615 1] Save Player Data
    (bind _asmario_party_gmi (Utilities|Casting|CastToMarioPartyGMI (Game|GetGameInstance)))
    (Default|SetPlayerData _asmario_party_gmi (Variables|/Game/Blueprints/TileMap.TileMap_C|GetCurrent%20Index (Variables|Default|GetTileMap)) _currenttile (Variables|Default|GetCoins) (Variables|Default|GetStars) (Variables|Default|GetCurrentDirection) (Variables|/Game/Blueprints/Tile.Tile_C|GetCoord _currenttile))
    (Default|ChangePlayer (Variables|Default|GetCurrentTile))
    (bind _outactors_2 (Actor|GetAllActorsOfClass "PlayerParty_C"))
    (Variables|PlayerParty_C|SetActual%20Player (Utilities|Array|Get(acopy) _outactors_2 (Variables|/Game/Blueprints/TileMap.TileMap_C|GetCurrent%20Index (Variables|Default|GetTileMap))) true)
    (if (== (Variables|/Game/Blueprints/TileMap.TileMap_C|GetCurrent%20Index (Variables|Default|GetTileMap)) 0)
      (Variables|PlayerParty_C|SetActual%20Player (Utilities|Array|Get(acopy) _outactors_2 (LocalVariables|Get3rdPlayer)) false)
      (else
        (Variables|PlayerParty_C|SetActual%20Player (Utilities|Array|Get(acopy) _outactors_2 (- (Variables|/Game/Blueprints/TileMap.TileMap_C|GetCurrent%20Index (Variables|Default|GetTileMap)) 1)) false)))
    (if (== (Variables|/Game/Blueprints/TileMap.TileMap_C|GetCurrent%20Index (Variables|Default|GetTileMap)) 0)
      (Game|OpenLevel(byObjectReference) "/Game/Levels/JumpMinigameMap.JumpMinigameMap"))
    (elif (== (Utilities|GetClass (Variables|Default|GetCurrentTile)) "/Game/Blueprints/Tiles/RedTile.RedTile_C")
      (if (<= (Variables|Default|GetCoins) 3)
        (Variables|Default|SetCoins 0)
        (goto _label)
        (else
          (bind _output_get_2 (Variables|Default|SetCoins (- (Variables|Default|GetCoins) 3)))
          (Development|PrintString (Utilities|String|Append "Perdiste 3 Monedas tienes" (Utilities|String|ToString(Integer) _output_get_2)))
          (goto _label)))
      (elif (== (Utilities|GetClass (Variables|Default|GetCurrentTile)) "/Game/Blueprints/Tiles/StarTile.StarTile_C")
        (if (>= (Variables|Default|GetCoins) 20)
          (bind _returnvalue (UserInterface|CreateWidget "/Game/Blueprints/BuyStore.BuyStore_C"))
          (bind _output_get_3 (Variables|Default|SetBuyUI _returnvalue))
          (UserInterface|Viewport|AddtoViewport _output_get_3 0))))))