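; Shared camera for Minigame2 that zooms to the spread of two to four players.
; After a short delay it caches the MinigameGM player list and becomes the view target for player controllers.
; A fast looping timer sets spring arm length to the largest checked player-to-player distance, clamped between min and max.
; The four-player check omits the P2–P4 pair.
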(event Custom|UpdateCamera
  (switch int (Utilities|Array|Length (Variables|Default|GetLocalPlayersVar))
    (:2
      (CallFunction|SetArmLengthP2))
    (:3
      (CallFunction|SetArmLengthP3))
    (:4
      (CallFunction|SetArmLengthP4))))

(event EventBeginPlay
  (Utilities|FlowControl|Delay 0.1)
  (CallFunction|ClassSetup)
  (Utilities|Time|SetTimerbyFunctionName 0 "UpdateCamera" 0.001 true))

(fn ConstructionScript)

(fn ClassSetup
  (bind _asminigame_gm (Utilities|Casting|CastToMinigameGM (Game|GetGameMode)))
  (bind _output_get (Variables|Default|SetAs%20Minigame%20GM _asminigame_gm))
  (Variables|Default|SetLocalPlayersVar (Variables|/Game/Minigame2/MinigameGM.MinigameGM_C|GetAllPlayers _output_get))
  (bind _outactors (Actor|GetAllActorsOfClass "/Script/Engine.PlayerController"))
  (Game|Player|SetViewTargetwithBlend _outactors self 0.0 "VTBlend_Linear" 0.0 false)
  (for (_array_element _array_index) (Variables|Default|GetLocalPlayersVar)
    (switch int _array_index
      (:0
        (Variables|Default|Setp1 _array_element))
      (:1
        (Variables|Default|Setp2 _array_element))
      (:2
        (Variables|Default|Setp3 _array_element))
      (:3
        (Variables|Default|Setp4 _array_element)))))

(fn SetArmLengthP4
  (bind _p1 (Variables|Default|Getp1))
  (bind _p2 (Variables|Default|Getp2))
  (bind _p3 (Variables|Default|Getp3))
  (bind _p4 (Variables|Default|Getp4))
  (Variables|/Script/Engine.SpringArmComponent|SetTargetArmLength (Variables|Default|GetSpringArm) (Math|Float|Clamp(Float) (.MaxValue (Math|Float|MaxOfFloatArray (Utilities|Array|MakeArray (Transformation|GetDistanceTo _p1 _p2) (Transformation|GetDistanceTo _p1 _p3) (Transformation|GetDistanceTo _p2 _p3) (Transformation|GetDistanceTo _p3 _p4) (Transformation|GetDistanceTo _p2 _p3) (Transformation|GetDistanceTo _p1 _p4)))) (Variables|Default|GetMinArmLength) (Variables|Default|GetMaxArmLength))))

(fn SetArmLengthP3
  (bind _p1 (Variables|Default|Getp1))
  (bind _p2 (Variables|Default|Getp2))
  (bind _p3 (Variables|Default|Getp3))
  (Variables|/Script/Engine.SpringArmComponent|SetTargetArmLength (Variables|Default|GetSpringArm) (Math|Float|Clamp(Float) (.MaxValue (Math|Float|MaxOfFloatArray (Utilities|Array|MakeArray (Transformation|GetDistanceTo _p1 _p2) (Transformation|GetDistanceTo _p1 _p3) (Transformation|GetDistanceTo _p2 _p3) (Transformation|GetDistanceTo _p2 _p3)))) (Variables|Default|GetMinArmLength) (Variables|Default|GetMaxArmLength))))

(fn SetArmLengthP2
  (Variables|/Script/Engine.SpringArmComponent|SetTargetArmLength (Variables|Default|GetSpringArm) (Math|Float|Clamp(Float) (Transformation|GetDistanceTo (Variables|Default|Getp1) (Variables|Default|Getp2)) (Variables|Default|GetMinArmLength) (Variables|Default|GetMaxArmLength))))